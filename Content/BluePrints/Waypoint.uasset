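; Waypoint actor that forms one link in an ordered chain of waypoints, grouped by a RangeID.
; On BeginPlay it searches all Waypoint actors and stores the one with the same RangeID and the next Order value as NextWaypoint.
; The chain therefore builds itself at runtime from those two variables, with no overlap, tick or construction logic.
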(event `self.ReceiveBeginPlay`
  (bind _outactors (`GameplayStatics.GetAllActorsOfClass` "Waypoint_C"))
  (for _array_element _outactors
    (if (and (== (`/Game/BluePrints/Waypoint.RangeID` _array_element) (`self.RangeID`)) (== (+ (`self.Order`) 1) (`/Game/BluePrints/Waypoint.Order` _array_element)))
      (set `self.nextWaypoint` _array_element))))

(fn `UserConstructionScript`)