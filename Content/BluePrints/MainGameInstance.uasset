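; MainGameInstance is the game instance that handles multiplayer sessions and holds the player's name.
; Hosting creates an eight-slot LAN session, then opens the arena level as a listen server, or quits the game if creation fails.
; Joining passes a chosen server-list result to JoinSession.
; On Init it loads the player name from the settings save slot, falling back to a default.
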(event `HostGameEvent`
  (`CreateSessionCallbackProxy.CreateSession` (`GameplayStatics.GetPlayerController` 0) 8 true
    (:`OnSuccess`
      (`GameplayStatics.OpenLevel` "low_poly_arena" true "listen"))
    (:`OnFailure`
      (`KismetSystemLibrary.ExecuteConsoleCommand` "quit"))))

(event `JoinFromServerListEvent`
  (params (server :type "BlueprintSessionResult Structure"))
  (`JoinSessionCallbackProxy.JoinSession` (`GameplayStatics.GetPlayerController` 0) server))

(event `self.ReceiveInit`
  (bind _returnvalue (`GameplayStatics.LoadGameFromSlot` "settings"))
  (bind _asmain_save (cast `/Game/BluePrints/MainSave` _returnvalue)
    (:`then`
      (set `self.playerName` (`/Game/BluePrints/MainSave.PlayerName` _asmain_save)))
    (:`CastFailed`
      (set `self.playerName` "Player"))))