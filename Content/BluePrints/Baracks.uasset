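; Barracks actor that periodically spawns waves of Chibi_creep units for its team.
; BeginPlay spawns a wave immediately, then starts a looping timer for the following waves.
; On authority only, each wave calls effectBroadcast to activate the particle system, then after a short delay spawns three creeps at scene-component points, passing Team, RangeId and fixed stats.
; Spawns at three further points are unconnected and never run.
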(event `effectBroadcast`
  (`ActorComponent.Activate` (`self.ParticleSystem`) true))

(event `spawnCreeps`
  (`/Engine/EditorBlueprintResources/ActorMacros.Switch Has Authority`
    (:`Authority`
      (`self.effectBroadcast`)
      (`KismetSystemLibrary.Delay` 0.3)
      (`|SpawnActorFromClass` "/Game/Units/Creeps/Chibi_creep.Chibi_creep_C" (`SceneComponent.K2_GetComponentToWorld` (`self.Scene`)) "Undefined" "OverrideRootScale" null (`self.team`) 100.0 0.0 10.0 (`self.rangeId`))
      (`|SpawnActorFromClass` "/Game/Units/Creeps/Chibi_creep.Chibi_creep_C" (`SceneComponent.K2_GetComponentToWorld` (`self.Scene4`)) "Undefined" "OverrideRootScale" null (`self.team`) 100.0 0.0 10.0 (`self.rangeId`))
      (`|SpawnActorFromClass` "/Game/Units/Creeps/Chibi_creep.Chibi_creep_C" (`SceneComponent.K2_GetComponentToWorld` (`self.Scene1`)) "Undefined" "OverrideRootScale" null (`self.team`) 100.0 0.0 10.0 (`self.rangeId`)))))

(event `self.ReceiveBeginPlay`
  (`self.spawnCreeps`)
  (`KismetSystemLibrary.K2_SetTimer` self "spawnCreeps" 25.0 true))

(fn `UserConstructionScript`)