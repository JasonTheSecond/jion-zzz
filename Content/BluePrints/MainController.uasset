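; Player controller that handles team choice and character spawning.
; On BeginPlay, the server spawns and possesses a SpectatorPawn at a team 0 spawn point.
; The teamOne and teamTwo inputs set Team, then spawn and possess a Chibi_Character with preset stats at that team's spawn.
; Despite its name, GetRandomSpawn picks the last TeamSpawn actor matching the team, with no randomization.
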(event `SetTeam`
  (params (team :type Integer))
  (set `self.team` team))

(event `InputAction|teamTwo`
  (params (Key :type "Key Structure" :default "AnyKey"))
  (:`Pressed`
    (`self.SetTeam` 2)
    (`self.Spawn` :!label _label)))

(event `InputAction|teamOne`
  (params (Key :type "Key Structure" :default "AnyKey"))
  (:`Pressed`
    (`self.SetTeam` 1)
    (goto _label)))

(event `Spawn`
  (bind _team (`self.team`))
  (bind _spawnoutput (`self.getRandomSpawn` _team))
  (bind _returnvalue (`|SpawnActorFromClass` "/Game/Chibi_characters/Chibi_Character.Chibi_Character_C" (`self.GetTransform` _spawnoutput) "Undefined" "OverrideRootScale" null _team 100.0 0.0 50.0))
  (`self.Possess` _returnvalue))

(event `self.ReceiveBeginPlay`
  (`/Engine/EditorBlueprintResources/ActorMacros.Switch Has Authority`
    (:`Authority`
      (bind _spawnoutput (`self.getRandomSpawn` 0))
      (bind _returnvalue (`|SpawnActorFromClass` "/Script/Engine.SpectatorPawn" (`self.GetTransform` _spawnoutput) "Undefined" "OverrideRootScale"))
      (`self.Possess` _returnvalue))))

(fn `getRandomSpawn`
  (params (team :type Integer))
  (returns (spawnOutput :type "/Game/BluePrints/TeamSpawn Object Reference"))
  (locals (playerSpawn :type "/Game/BluePrints/TeamSpawn Object Reference"))
  (bind _outactors (`GameplayStatics.GetAllActorsOfClass` "/Game/BluePrints/TeamSpawn.TeamSpawn_C"))
  (for _array_element _outactors
    (if (== (`/Game/BluePrints/TeamSpawn.team` _array_element) team)
      (set `local.playerSpawn` _array_element)))
  (return (`local.playerSpawn`)))

(fn `UserConstructionScript`)